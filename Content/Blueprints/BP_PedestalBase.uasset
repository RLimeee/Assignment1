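; BP_PedestalBase is a pedestal Blueprint with a point light that switches between an on color and an off color.
; TurnLightOnOrOff sets the light to OnColor or OffColor, changing only color, not visibility or intensity.
; ToggleLight stores no state flag: it infers the state by comparing the current light color to OnColor within a small tolerance, then applies the opposite.
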(fn `ToggleLight`
  (`self.Turn Light On or Off` (not (`KismetMathLibrary.LinearColor_IsNearEqual` (`self.OnColor`) (`LightComponentBase.GetLightColor` (`self.PointLight`)) 0.001))))

(fn `Turn Light On or Off`
  (params (`ShouldTurnOn?` :type Boolean))
  (if `ShouldTurnOn?`
    (`LightComponent.SetLightColor` (`self.PointLight`) (`self.OnColor`) true)
    (else
      (`LightComponent.SetLightColor` (`self.PointLight`) (`self.OffColor`) true))))

(fn `UserConstructionScript`)