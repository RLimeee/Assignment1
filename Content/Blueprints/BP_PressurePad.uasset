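; BP_PressurePad is a pressure pad that sinks when something overlaps its Box collision and rises when the overlap ends.
; Begin and end overlap set the OnOf flag, print a debug string, and play or reverse the MoveDown timeline.
; Each timeline update offsets the PressurePad mesh's relative Z and calls the PressedonOff event dispatcher with OnOf, so listeners hear it throughout the animation rather than only on completion.
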(event `self.Box.OnComponentBeginOverlap`
  (params (OverlappedComponent :type "PrimitiveComponent Object Reference") (OtherActor :type "Actor Object Reference") (OtherComp :type "PrimitiveComponent Object Reference") (OtherBodyIndex :type Integer) (bFromSweep :type Boolean) (SweepResult :type "HitResult Structure (by ref)"))
  ;[1 1 1] Add a collision volume and adjust its placement in the viewport (watch out for which component it's attached to since the PressurePad Mesh will be moving but we don't want the collision volume moving with it). Add ComponentBeginOverlap and ComponentEndOverlap events for the collision component here. Create an Event Dispatcher in this class. Call that event when the pressure pad is finished animating and call the event dispatcher passing the correct true or false value based on whether it was just played forward or backward.
  (`KismetSystemLibrary.PrintString` "on")
  (set `self.On Of` true)
  (bind (_direction _movedown) (`Timeline|MoveDown` :!label _label)
    (:`Update`
      (`SceneComponent.K2_SetRelativeLocation` (`self.PressurePad`) (`KismetMathLibrary.MakeVector` 0.0 0.0 (* _movedown -10.0)) false false)
      (`self.pressedonOff` (`self.On Of`)))))

(event `self.Box.OnComponentEndOverlap`
  (params (OverlappedComponent :type "PrimitiveComponent Object Reference") (OtherActor :type "Actor Object Reference") (OtherComp :type "PrimitiveComponent Object Reference") (OtherBodyIndex :type Integer))
  ;[1 1 1] Add a collision volume and adjust its placement in the viewport (watch out for which component it's attached to since the PressurePad Mesh will be moving but we don't want the collision volume moving with it). Add ComponentBeginOverlap and ComponentEndOverlap events for the collision component here. Create an Event Dispatcher in this class. Call that event when the pressure pad is finished animating and call the event dispatcher passing the correct true or false value based on whether it was just played forward or backward.
  (`KismetSystemLibrary.PrintString` "off")
  (set `self.On Of` false)
  (goto _label :!via `Reverse`))

(fn `UserConstructionScript`)