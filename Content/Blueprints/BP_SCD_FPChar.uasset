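; First-person player character with movement, mouse and gamepad look, double jump and widget clicking.
; Interact sphere-traces 200 units along the view and messages any hit actor implementing BPI_Interact.
; Double jump launches along current input relative to facing, once per airtime, while crouching blocks jumping.
; Footstep and landing sounds follow floor surface type, with landings adding a camera shake that varies after a double jump.
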(event `InputAction|Interact`
  (params (Key :type "Key Structure"))
  (bind (_outlocation _outrotation) (`self.GetActorEyesViewPoint`))
  ;[1 0.8515 0] Add Sphere Trace in front of the character for ButtonPedestal. If a valid object is found, send it the Interact message.
  (:`Pressed`
    (bind _outhit (`KismetSystemLibrary.SphereTraceSingle` :`Start` _outlocation :`End` (+ _outlocation (* (`KismetMathLibrary.Conv_RotatorToVector` _outrotation) 200.0)) :`Radius` (`CapsuleComponent.GetUnscaledCapsuleRadius` (`self.CapsuleComponent`)) :`TraceChannel` "TraceTypeQuery1" :`bTraceComplex` true :`DrawDebugType` "ForDuration" :`DrawTime` 0.5))
    (bind (_bblockinghit _binitialoverlap _time _distance _location _impactpoint _normal _impactnormal _physmat _hitactor) (`GameplayStatics.BreakHitResult` _outhit))
    (if (`KismetSystemLibrary.DoesImplementInterface` _hitactor "/Game/Blueprints/BPI_Interact.BPI_Interact_C")
      (message `/Game/Blueprints/BPI_Interact.Send Function` _hitactor))))

(event `InputAxis|Move Forward / Backward`
  (params (AxisValue :type "Float (single-precision)"))
  ;[1 1 1] Ignore: Movement input
  (bind _output_get (set `self.ForwardAxisValue` AxisValue))
  (`self.AddMovementInput` (`self.GetActorForwardVector`) _output_get)
  ;[1 1 1] Ignore: Playing footstep sounds
  (if (`self.IsWalkingOnTheGround`) :!label _label
    (`KismetSystemLibrary.Delay` 0.07)
    (bind _surfacetype (`self.GetSurfaceType`)
      (:`  `
        (`self.ProcessFootstepSound` _surfacetype)))))

(event `InputAxis|Move Right / Left`
  (params (AxisValue :type "Float (single-precision)"))
  ;[1 1 1] Ignore: Movement input
  (bind _output_get (set `self.SidewaysAxisValue` AxisValue))
  (`self.AddMovementInput` (`self.GetActorRightVector`) _output_get)
  (goto _label))

(event `InputAxis|Turn Right / Left Mouse`
  (params (AxisValue :type "Float (single-precision)"))
  ;[1 1 1] Ignore: Mouse camera control
  (`self.AddControllerYawInput` (* (* AxisValue (`GameplayStatics.GetWorldDeltaSeconds`)) (`self.MouseSensetivity`))))

(event `InputAxis|Turn Right / Left Gamepad`
  (params (AxisValue :type "Float (single-precision)"))
  ;[1 1 1] Ignore: Joystick camera control
  (`self.AddControllerYawInput` (* AxisValue (`self.BaseTurnRate`) (`GameplayStatics.GetWorldDeltaSeconds`))))

(event `Key|LeftMouseButton`
  (params (Key :type "Key Structure"))
  (bind _widgetinteraction (`self.WidgetInteraction`))
  ;[1 1 1] Ignore: Mouse Buttons Input
  (:`Pressed`
    (`WidgetInteractionComponent.PressPointerKey` _widgetinteraction Key))
  (:`Released`
    (`WidgetInteractionComponent.ReleasePointerKey` _widgetinteraction Key)))

(event `Key|RightMouseButton`
  (params (Key :type "Key Structure"))
  (bind _widgetinteraction (`self.WidgetInteraction`))
  ;[1 1 1] Ignore: Mouse Buttons Input
  (:`Pressed`
    (`WidgetInteractionComponent.PressPointerKey` _widgetinteraction Key))
  (:`Released`
    (`WidgetInteractionComponent.ReleasePointerKey` _widgetinteraction Key)))

(event `InputAxis|Look Up / Down Mouse`
  (params (AxisValue :type "Float (single-precision)"))
  ;[1 1 1] Ignore: Mouse camera control
  (`self.AddControllerPitchInput` (* (* (`GameplayStatics.GetWorldDeltaSeconds`) AxisValue) (`self.MouseSensetivity`))))

(event `InputAxis|Look Up / Down Gamepad`
  (params (AxisValue :type "Float (single-precision)"))
  ;[1 1 1] Ignore: Joystick camera control
  (`self.AddControllerPitchInput` (* AxisValue (`self.BaseLookUpRate`) (`GameplayStatics.GetWorldDeltaSeconds`))))

(event `self.OnLanded`
  (params (Hit :type "HitResult Structure (by ref)"))
  ;[1 1 1] Ignore: Play landing sound
  (`self.ProcessFootstepSound` (`GameplayStatics.GetSurfaceType` Hit) true))

(event `InputAction|Jump` :overrideparent false
  (params (Key :type "Key Structure"))
  ;[1 1 1] Ignore: Jump
  (:`Pressed`
    (if (not (`self.bCrouchKeyIsHeld`))
      (if (`CharacterMovementComponent.IsWalking` (`self.CharacterMovement`))
        (`GameplayStatics.SpawnSoundAttached` "/Game/SuperGrid/TutorialLevel/SoundEffects/Cue_Jump.Cue_Jump" (`self.CapsuleComponent`) "None" (0.0 0.0 0.0) (struct) "KeepRelativeOffset" false 1.0 1.0 0.0 null null)
        (`self.Jump`)
        (elif (not (`self.bDoubleJumped`))
          (`self.DoubleJump`)))))
  (:`Released`
    (`self.StopJumping`)))

(fn `CanJumpInternal`
  (returns (ReturnValue :type Boolean))
  (bind _returnvalue (`parent.CanJumpInternal`))
  (return (and _returnvalue (not (`self.bIsCrouching`)))))

(fn `DoubleJump`
  (bind _charactermovement (`self.CharacterMovement`))
  (bind _returnvalue (`MovementComponent.GetMaxSpeed` _charactermovement))
  ;[0.2979 0.7963 1] Apply created vector and play sound
  (`self.LaunchCharacter` (`KismetMathLibrary.TransformDirection` (`self.GetTransform`) (`KismetMathLibrary.MakeVector` (* (`self.ForwardAxisValue`) _returnvalue) (* (`self.SidewaysAxisValue`) _returnvalue) (`CharacterMovementComponent.JumpZVelocity` _charactermovement))) true true)
  (`GameplayStatics.SpawnSoundAttached` "/Game/SuperGrid/TutorialLevel/SoundEffects/Cue_DoubleJump.Cue_DoubleJump" (`self.CapsuleComponent`) "None" (0.0 0.0 0.0) (struct) "KeepRelativeOffset" false 1.0 1.0 0.0 null null)
  ;[1 0.0495 0.03995] Disable any triple jumps and etc
  (set `self.bDoubleJumped` true))

(fn `ProcessFootstepSound`
  (params (SurfaceType :type "EPhysicalSurface Enum" :default "SurfaceType_Default") (bIsLanding :type Boolean))
  (locals (NewLocalVar_0 :type "SoundBase Object Reference" :default null) (bLanding :type Boolean) (lLanding :type Boolean))
  ;[0.845 0.5886 0.2746] Play sound for landing or basic footstep: depends on currect action
  (bind _output_get (set `local.lLanding` bIsLanding))
  (`GameplayStatics.SpawnSoundAttached` (select `EPhysicalSurface` SurfaceType :`SurfaceType_Default` (select `bool` _output_get :`false` "/Game/SuperGrid/TutorialLevel/SoundEffects/Cue_Footstep.Cue_Footstep" :`true` "/Game/SuperGrid/TutorialLevel/SoundEffects/Cue_Landing.Cue_Landing" :!type "SoundBase Object Reference")) (`self.CapsuleComponent`) "None" (0.0 0.0 0.0) (struct) "KeepRelativeOffset" false 0.7 1.0 0.0 null null)
  ;[0.2569 0.1653 0.57] Play Camera shake on Landing
  (if (`local.lLanding`)
    (`GameplayStatics.PlayWorldCameraShake` (select `bool` (`self.bDoubleJumped`) :!type "MatineeCameraShake Class Reference") (`SceneComponent.K2_GetComponentLocation` (`self.CapsuleComponent`)) 1.0 500.0)
    (set `self.bDoubleJumped` false)))

(fn `UserConstructionScript`
  (set `self.UserHeight` (`CapsuleComponent.GetScaledCapsuleHalfHeight` (`self.CapsuleComponent`))))